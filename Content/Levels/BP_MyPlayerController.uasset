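; Player controller that relays camera input to the possessed CB_CameraController pawn, which it casts to on each input event.
; Orbit, forward and strafe axes pass their values straight through, while the zoom in and out actions send fixed opposite steps to CameraZoom on press.
; The pawn's functions do the actual camera work, and a leftover SpawnBuilding call is never executed.
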(event EventBeginPlay)

(event Input|ActionEvents|InputActionCameraZoomIn
  (params (Key :type Key%20Structure))
  (:Pressed
    (bind _ascb_camera_controller (Utilities|Casting|CastToCB_CameraController (Pawn|GetControlledPawn)))
    (Default|CameraZoom _ascb_camera_controller -1.0)))

(event Input|ActionEvents|InputActionCameraZoomOut
  (params (Key :type Key%20Structure))
  (:Pressed
    (bind _ascb_camera_controller (Utilities|Casting|CastToCB_CameraController (Pawn|GetControlledPawn)))
    (Default|CameraZoom _ascb_camera_controller 1.0)))

(event Input|AxisEvents|InputAxisCameraOrbit
  (params (AxisValue :type Float%20%28single-precision%29))
  (bind _ascb_camera_controller (Utilities|Casting|CastToCB_CameraController (Pawn|GetControlledPawn)))
  (Default|CameraOrbit _ascb_camera_controller AxisValue))

(event Input|AxisEvents|InputAxisMoveForward
  (params (AxisValue :type Float%20%28single-precision%29))
  (bind _ascb_camera_controller (Utilities|Casting|CastToCB_CameraController (Pawn|GetControlledPawn)))
  (Default|MoveForward _ascb_camera_controller AxisValue))

(event Input|AxisEvents|InputAxisStrafeLeft/Right
  (params (AxisValue :type Float%20%28single-precision%29))
  (bind _ascb_camera_controller (Utilities|Casting|CastToCB_CameraController (Pawn|GetControlledPawn)))
  (Default|Left/RightStrafe _ascb_camera_controller AxisValue))

(event Input|KeyboardEvents|SpaceBar
  (params (Key :type Key%20Structure)))

(fn ConstructionScript)