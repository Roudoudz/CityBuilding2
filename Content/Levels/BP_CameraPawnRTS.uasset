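; RTS-style camera pawn that lets the player pan, orbit and zoom the view through input axis events.
; Forward and strafe input move the pawn along directions built from control yaw only, so pitch does not affect movement.
; Orbit adds controller yaw scaled by OrbitSpeed.
; Zoom adjusts the CameraArm length by ZoomSpeed, clamped between ZoomMin and ZoomMax.
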(event Custom|CameraOrbit
  (params (Magnitude :type Float%20%28single-precision%29))
  (Pawn|Input|AddControllerYawInput (* Magnitude (Variables|Default|GetOrbitSpeed))))

(event Custom|MoveForward
  (params (Magnitude :type Float%20%28single-precision%29))
  (Pawn|Input|AddMovementInput (Math|Vector|GetForwardVector (Math|Rotator|MakeRotator 0.0 0.0 (.Yaw (Math|Rotator|BreakRotator (Pawn|GetControlRotation :!class /Script/Engine.Pawn))))) Magnitude false))

(event Custom|Left/RightStrafe
  (params (Magnitude :type Float%20%28single-precision%29))
  (Pawn|Input|AddMovementInput (Math|Vector|GetRightVector (Math|Rotator|MakeRotator 0.0 0.0 (.Yaw (Math|Rotator|BreakRotator (Pawn|GetControlRotation :!class /Script/Engine.Pawn))))) Magnitude false))

(event Custom|CameraZoom
  (params (Magnitude :type Float%20%28single-precision%29))
  (bind _cameraarm (Variables|Default|GetCameraArm))
  (Variables|/Script/Engine.SpringArmComponent|SetTargetArmLength _cameraarm (Math|Float|Clamp(Float) (+ (* Magnitude (Variables|Default|GetZoomSpeed)) (Variables|/Script/Engine.SpringArmComponent|GetTargetArmLength _cameraarm)) (Variables|Default|GetZoomMin) (Variables|Default|GetZoomMax))))

(event EventBeginPlay)

(fn ConstructionScript)